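; Snow deformation capture actor that follows a player vehicle in texel-snapped XY steps to keep the scene capture stable.
; On BeginPlay it clears both render targets and publishes the capture size to MPC_Capture.
; Each Tick it moves, publishes its location, then draws M_DrawToPersistent into RT_Persistent with the normalized move offset, so accumulated deformation scrolls with it.
; PlayerVehicle is not assigned in any executed path here.
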(event EventBeginPlay
  (Rendering|Material|SetScalarParameterValue "/Game/SnowDeformation/Materials/MPC_Capture.MPC_Capture" "CaptureSize" (Variables|/Script/Engine.SceneCaptureComponent2D|GetOrthoWidth (Variables|Default|GetSceneCapture)) :!class /Script/Engine.KismetMaterialLibrary)
  (bind _returnvalue (Rendering|Material|CreateDynamicMaterialInstance "/Game/SnowDeformation/Materials/M_DrawToPersistent.M_DrawToPersistent" "None" :!class /Script/Engine.KismetMaterialLibrary))
  (Variables|Default|SetDrawMaterial _returnvalue)
  (Rendering|ClearRenderTarget2D "/Game/SnowDeformation/RenderTargets/RT_Capture.RT_Capture")
  (Rendering|ClearRenderTarget2D "/Game/SnowDeformation/RenderTargets/RT_Persistent.RT_Persistent"))

(event EventTick
  (params (DeltaSeconds :type Float%20%28single-precision%29))
  (CallFunction|MoveCapture)
  (CallFunction|DrawtoPersistent))

(fn ConstructionScript)

(fn DrawtoPersistent
  (bind _scenecapture (Variables|Default|GetSceneCapture))
  (bind _moveoffset (Variables|Default|GetMoveOffset))
  (bind _orthowidth (Variables|/Script/Engine.SceneCaptureComponent2D|GetOrthoWidth _scenecapture))
  (bind _returnvalue (/ _moveoffset _orthowidth))
  (Rendering|Material|SetVectorParameterValue (Variables|Default|GetDrawMaterial) "Offset" (Utilities|Struct|MakeLinearColor (.x _returnvalue) (.y _returnvalue) 0.0 1.0) :!class /Script/Engine.MaterialInstanceDynamic)
  (Rendering|DrawMaterialtoRenderTarget "/Game/SnowDeformation/RenderTargets/RT_Persistent.RT_Persistent" (Variables|Default|GetDrawMaterial)))

(fn MoveCapture
  (bind _returnvalue (Transformation|GetActorLocation))
  (bind _returnvalue_2 (/ 1.0 2048.0))
  (bind _playervehicle (Variables|Default|GetPlayerVehicle))
  (bind _scenecapture (Variables|Default|GetSceneCapture))
  (bind _returnvalue_3 (Transformation|GetActorLocation _playervehicle))
  (bind _orthowidth (Variables|/Script/Engine.SceneCaptureComponent2D|GetOrthoWidth _scenecapture))
  (bind _returnvalue_4 (* _orthowidth _returnvalue_2))
  (bind _returnvalue_5 (Utilities|SnaptoPixelWorldSize (.x _returnvalue_3) (.y _returnvalue_3) _returnvalue_4))
  (bind _returnvalue_6 (- _returnvalue_5 _returnvalue))
  (Utilities|IsValid _playervehicle
    (:Is%20Valid
      (bind _output_get (Variables|Default|SetMoveOffset (Math|Vector2D|MakeVector2D (.x _returnvalue_6) (.y _returnvalue_6))))
      (Transformation|AddActorWorldOffset (Math|Vector|MakeVector (.x _output_get) (.y _output_get) 0.0))
      (Rendering|Material|SetVectorParameterValue "/Game/SnowDeformation/Materials/MPC_Capture.MPC_Capture" "CaptureLocation" (Math|Conversions|ToLinearColor(Vector) (Transformation|GetActorLocation)) :!class /Script/Engine.KismetMaterialLibrary))
    (:Is%20Not%20Valid
      (Development|PrintString "No Valid Char"))))
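; HexTileManager hands out team ownership of the hex map's start tiles.
; When the UpdateStartTiles flag is set, its construction script adds every HexTile marked StartTile to an array, shuffles it and assigns each index as OwningTeam.
; It calls UpdateStartTiles on each tile, then clears the flag, so the flag works as a one-shot trigger.
; The event graph holds only an unconnected copy of this logic.
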(event EventBeginPlay)

(event Collision|EventActorBeginOverlap
  (params (OtherActor :type Actor%20Object%20Reference)))

(event EventTick
  (params (DeltaSeconds :type Float%20%28single-precision%29)))

(fn ConstructionScript
  (bind _starttiles (Variables|Default|GetStartTiles))
  (if (Variables|Default|GetUpdateStartTiles)
    (bind _outactors (Actor|GetAllActorsOfClass "/Game/Blueprints/HexTile.HexTile_C"))
    (for _array_element _outactors
      (if (Variables|/Game/Blueprints/HexTile.HexTile_C|GetStartTile? _array_element)
        (Utilities|Array|AddUnique (Variables|Default|GetStartTiles) _array_element)))
    (Utilities|Array|Shuffle _starttiles)
    (for (_array_element_2 _array_index) _starttiles
      (Variables|/Game/Blueprints/HexTile.HexTile_C|SetOwningTeam _array_element_2 _array_index)
      (Default|UpdateStartTiles _array_element_2))
    (Variables|Default|SetUpdateStartTiles false)))
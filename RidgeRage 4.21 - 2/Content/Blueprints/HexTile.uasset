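; Capturable hex tile that vehicles claim for their team by driving over it.
; On the server, overlap claims an unowned tile or neutralizes one held by another team.
; OnRep functions for owner and team set material color from a team color collection and run timelines animating fill and outline, locking capture until finished.
; Construction script previews ownership and makes start tiles locked, with glow and arrow facing the start tiles' average location.
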(event OnComponentBeginOverlap(HexTile_Collider)
  (params (OverlappedComponent :type Primitive%20Component%20Object%20Reference) (OtherActor :type Actor%20Object%20Reference) (OtherComp :type Primitive%20Component%20Object%20Reference) (OtherBodyIndex :type Integer) (bFromSweep :type Boolean) (SweepResult :type Hit%20Result%20Structure%20%28by%20ref%29))
  (Networking|SwitchHasAuthority
    (:Authority
      (if (Variables|Default|GetCanChangeTeam?)
        (bind _asvehicle_blueprint (Utilities|Casting|CastToVehicleBlueprint OtherActor))
        (if (Variables|Default|GetOwned?)
          (if (not (== (Variables|Default|GetOwningTeam) (Variables|/Game/VehicleAdvBP/Blueprints/VehicleBlueprint.VehicleBlueprint_C|GetTeamNumber _asvehicle_blueprint)))
            (Variables|Default|SetOwned? false))
          (else
            (Variables|Default|SetOwningTeam (Variables|/Game/VehicleAdvBP/Blueprints/VehicleBlueprint.VehicleBlueprint_C|GetTeamNumber _asvehicle_blueprint))
            (Variables|Default|SetOwned? true)))))))

(event Custom|UpdateStartTiles
  (bind _hextile (Variables|Components|GetHexTile))
  ;[1 1 1] Gets Color From Collection
  (bind _returnvalue (Rendering|Material|GetVectorParameterValue "/Game/Blueprints/MPC_TeamColors.MPC_TeamColors" (Utilities|Name|MakeLiteralName (Utilities|String|StringToName (Utilities|String|Append "Team" (Utilities|String|ToString(Integer) (+ (Variables|Default|GetOwningTeam) 1))))) :!class /Script/Engine.KismetMaterialLibrary))
  ;[1 1 1] Sets Color
  (Rendering|Material|SetVectorParameterValueonMaterials _hextile "OwningTeamColor" (Math|Conversions|ToVector(LinearColor) _returnvalue))
  ;[1 1 1] Sets Color Alpha
  (Rendering|Material|SetScalarParameterValueonMaterials _hextile "TileColorAlpha" 1.0)
  ;[1 1 1] Sets the Mask
  (Rendering|Material|SetScalarParameterValueonMaterials _hextile "ThickLineMask" 1e+02)
  ;[1 1 1] Sets the Width
  (Rendering|Material|SetScalarParameterValueonMaterials _hextile "ThickLineWidth" 4.0)
  (Rendering|SetVisibility (Variables|Default|GetStartTileEffect) true false)
  ;[1 1 1] Sets Color
  (Rendering|Material|SetVectorParameterValueonMaterials (Variables|Default|GetStartTileEffect) "Emissive Color" (* (Math|Conversions|ToVector(LinearColor) _returnvalue) 2.0))
  (Components|Arrow|SetArrowColor(LinearColor) (Variables|Default|GetArrow) _returnvalue)
  (bind _outactors (Actor|GetAllActorsOfClass "/Game/Blueprints/HexTileManager.HexTileManager_C"))
  (bind _returnvalue_2 (Class|GameplayStatics|GetActorArrayAverageLocation (Variables|/Game/Blueprints/HexTileManager.HexTileManager_C|GetStartTiles (Utilities|Array|Get(acopy) _outactors))))
  (bind _output_get (Variables|Default|SetFacingRotation (Math|Rotator|FindLookatRotation (Transformation|GetActorLocation) _returnvalue_2)))
  (Transformation|SetWorldRotation (Variables|Default|GetArrow) _output_get false false)
  (Rendering|Components|TextRender|SetText (Variables|Default|GetTextRender) (Utilities|Text|ToText(Integer) (Variables|Default|GetOwningTeam))))

(event Custom|Remove%20Owning%20Team
  (bind _hextile (Variables|Components|GetHexTile))
  (Variables|Default|SetCanChangeTeam? false)
  (bind (_direction _mask_track _width_track) (Timeline|Timeline_0 PlayFromStart)
    (:Update
      ;[1 1 1] Sets Color Alpha
      (Rendering|Material|SetScalarParameterValueonMaterials _hextile "TileColorAlpha" _mask_track)
      ;[1 1 1] Sets the Mask
      (Rendering|Material|SetScalarParameterValueonMaterials _hextile "ThickLineMask" (+ (* _mask_track 68.5) 31.5))
      ;[1 1 1] Sets the Width
      (Rendering|Material|SetScalarParameterValueonMaterials _hextile "ThickLineWidth" (+ (* _width_track 5.0) 4.0)))
    (:Finished
      (Variables|Default|SetCanChangeTeam? true))))

(event Custom|Set%20Tile%20Owned
  (bind _hextile (Variables|Components|GetHexTile))
  (Variables|Default|SetCanChangeTeam? false)
  (bind (_direction _mask_track _width_track) (Timeline|ForwardTimeline PlayFromStart)
    (:Update
      ;[1 1 1] Sets Color Alpha
      (Rendering|Material|SetScalarParameterValueonMaterials _hextile "TileColorAlpha" _mask_track)
      ;[1 1 1] Sets the Mask
      (Rendering|Material|SetScalarParameterValueonMaterials _hextile "ThickLineMask" (+ (* _mask_track 68.5) 31.5))
      ;[1 1 1] Sets the Width
      (Rendering|Material|SetScalarParameterValueonMaterials _hextile "ThickLineWidth" (+ (* _width_track 5.0) 4.0)))
    (:Finished
      (Variables|Default|SetCanChangeTeam? true))))

(event EventBeginPlay)

(event Collision|EventActorBeginOverlap
  (params (OtherActor :type Actor%20Object%20Reference)))

(event EventTick
  (params (DeltaSeconds :type Float%20%28single-precision%29)))

(fn ConstructionScript
  (bind _hextile (Variables|Components|GetHexTile))
  (if (Variables|Default|GetStartTile?)
    (CallFunction|UpdateStartTiles)
    (Variables|Default|SetCanChangeTeam? false)
    (Variables|Default|SetOwned? true))
  (if (Variables|Default|GetOwned?)
    ;[1 1 1] Gets Color From Collection
    (bind _returnvalue (Rendering|Material|GetVectorParameterValue "/Game/Blueprints/MPC_TeamColors.MPC_TeamColors" (Utilities|Name|MakeLiteralName (Utilities|String|StringToName (Utilities|String|Append "Team" (Utilities|String|ToString(Integer) (+ (Variables|Default|GetOwningTeam) 1))))) :!class /Script/Engine.KismetMaterialLibrary))
    ;[1 1 1] Sets Color
    (Rendering|Material|SetVectorParameterValueonMaterials _hextile "OwningTeamColor" (Math|Conversions|ToVector(LinearColor) _returnvalue))
    ;[1 1 1] Sets Color Alpha
    (Rendering|Material|SetScalarParameterValueonMaterials _hextile "TileColorAlpha" 1.0)
    ;[1 1 1] Sets the Mask
    (Rendering|Material|SetScalarParameterValueonMaterials _hextile "ThickLineMask" 1e+02)
    ;[1 1 1] Sets the Width
    (Rendering|Material|SetScalarParameterValueonMaterials _hextile "ThickLineWidth" 4.0)
    (else
      ;[1 1 1] Sets Color Alpha
      (Rendering|Material|SetScalarParameterValueonMaterials _hextile "TileColorAlpha" 0.0)
      ;[1 1 1] Sets the Mask
      (Rendering|Material|SetScalarParameterValueonMaterials _hextile "ThickLineMask" 31.5)
      ;[1 1 1] Sets the Width
      (Rendering|Material|SetScalarParameterValueonMaterials _hextile "ThickLineWidth" 4.0))))

(fn OnRepOwningTeam
  ;[1 1 1] Gets Color From Collection
  (bind _returnvalue (Rendering|Material|GetVectorParameterValue "/Game/Blueprints/MPC_TeamColors.MPC_TeamColors" (Utilities|Name|MakeLiteralName (Utilities|String|StringToName (Utilities|String|Append "Team" (Utilities|String|ToString(Integer) (+ (Variables|Default|GetOwningTeam) 1))))) :!class /Script/Engine.KismetMaterialLibrary))
  ;[1 1 1] Sets Color
  (Rendering|Material|SetVectorParameterValueonMaterials (Variables|Components|GetHexTile) "OwningTeamColor" (Math|Conversions|ToVector(LinearColor) _returnvalue)))

(fn OnRepOwned?
  (if (Variables|Default|GetOwned?)
    (CallFunction|SetTileOwned)
    (else
      (CallFunction|RemoveOwningTeam))))
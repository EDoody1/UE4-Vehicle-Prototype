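; VehicleGameState is a game state Blueprint that sets up team ownership of hex start tiles when play begins.
; On authority it gathers HexTile actors flagged as start tiles and shuffles them, then gives each its array index as owning team and updates it.
; Disconnected logic would randomly assign players to teams from a refillable pool; the team roll, start-tile assignment and Tick events are empty.
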(event Custom|Find%20and%20Assign%20Start%20Tiles)

(event Custom|Player%20Roll%20Team
  (params (NewParam :type Player%20Controller%20Object%20Reference)))

(event EventBeginPlay
  (bind _starttiles (Variables|Default|GetStartTiles))
  (Networking|SwitchHasAuthority
    (:Authority
      (bind _outactors (Actor|GetAllActorsOfClass "/Game/Blueprints/HexTile.HexTile_C"))
      (for _array_element _outactors
        (if (Variables|/Game/Blueprints/HexTile.HexTile_C|GetStartTile? _array_element)
          (Utilities|Array|AddUnique (Variables|Default|GetStartTiles) _array_element)))
      (Utilities|Array|Shuffle _starttiles))
    (:Remote
      (Development|PrintString "No Authority")))
  (for (_array_element_2 _array_index) _starttiles
    (Variables|/Game/Blueprints/HexTile.HexTile_C|SetOwningTeam _array_element_2 _array_index)
    (Default|UpdateStartTiles _array_element_2)))

(event EventTick
  (params (DeltaSeconds :type Float%20%28single-precision%29)))

(fn ConstructionScript)
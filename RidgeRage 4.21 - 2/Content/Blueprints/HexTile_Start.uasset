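; HexTile_Start is a team starting hex tile, a child Blueprint that sets CanChangeTeam to false.
; Its construction script shuffles all start tiles, assigns each an OwningTeam by index, and points FacingRotation0 at their average location.
; Construction and UpdateOwningTeam both look up the team's color by built parameter name in MPC_TeamColors and apply it, doubled, as the collider's emissive color.
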(event Custom|UpdateOwningTeam
  ;[1 1 1] Gets Color From Collection
  (bind _returnvalue (Rendering|Material|GetVectorParameterValue "/Game/Blueprints/MPC_TeamColors.MPC_TeamColors" (Utilities|Name|MakeLiteralName (Utilities|String|StringToName (Utilities|String|Append "Team" (Utilities|String|ToString(Integer) (+ (Variables|Default|GetOwningTeam) 1))))) :!class /Script/Engine.KismetMaterialLibrary))
  ;[1 1 1] Sets Color
  (Rendering|Material|SetVectorParameterValueonMaterials (Variables|Default|GetHexTile_Collider) "Emissive Color" (* (Math|Conversions|ToVector(LinearColor) _returnvalue) 2.0)))

(event EventBeginPlay
  (|CallParentFunction))

(event Collision|EventActorBeginOverlap
  (params (OtherActor :type Actor%20Object%20Reference))
  (|CallParentFunction OtherActor))

(event EventTick
  (params (DeltaSeconds :type Float%20%28single-precision%29))
  (|CallParentFunction DeltaSeconds))

(fn ConstructionScript
  (Variables|Default|SetCanChangeTeam? false)
  (bind _outactors (Actor|GetAllActorsOfClass "HexTile_Start_C"))
  (Utilities|Array|Shuffle _outactors)
  (for (_array_element _array_index) _outactors
    (Variables|/Game/Blueprints/HexTile.HexTile_C|SetOwningTeam _array_element _array_index))
  (bind _returnvalue (Class|GameplayStatics|GetActorArrayAverageLocation _outactors))
  (Variables|Default|SetFacingRotation_0 (Math|Rotator|FindLookatRotation (Transformation|GetActorLocation) _returnvalue))
  (|CallParentFunction)
  ;[1 1 1] Gets Color From Collection
  (bind _returnvalue_2 (Rendering|Material|GetVectorParameterValue "/Game/Blueprints/MPC_TeamColors.MPC_TeamColors" (Utilities|Name|MakeLiteralName (Utilities|String|StringToName (Utilities|String|Append "Team" (Utilities|String|ToString(Integer) (+ (Variables|Default|GetOwningTeam) 1))))) :!class /Script/Engine.KismetMaterialLibrary))
  ;[1 1 1] Sets Color
  (Rendering|Material|SetVectorParameterValueonMaterials (Variables|Default|GetHexTile_Collider) "Emissive Color" (* (Math|Conversions|ToVector(LinearColor) _returnvalue_2) 2.0)))
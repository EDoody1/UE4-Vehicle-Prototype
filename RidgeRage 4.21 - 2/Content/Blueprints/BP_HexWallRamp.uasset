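; BP_HexWallRamp is a hex tile wall piece whose shape is chosen by its WallType setting.
; The construction script switches on WallType to assign one of three wall meshes or a corner mesh to the HexTileCollider component, with a collider mesh for the missing-type case.
; An UpdateWallType event repeats the same switch so the mesh can be refreshed outside construction.
; The overlap event is an empty stub.
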(event OnComponentBeginOverlap(HexTile_Collider)
  (params (OverlappedComponent :type Primitive%20Component%20Object%20Reference) (OtherActor :type Actor%20Object%20Reference) (OtherComp :type Primitive%20Component%20Object%20Reference) (OtherBodyIndex :type Integer) (bFromSweep :type Boolean) (SweepResult :type Hit%20Result%20Structure%20%28by%20ref%29)))

(event Custom|UpdateWallType
  (bind _hextile_collider (Variables|Components|GetHexTile_Collider))
  (switch Utilities|FlowControl|Switch|SwitchonWallTypeEnum (Variables|Default|GetWall%20Type)
    (:NewEnumerator0
      (Components|StaticMesh|SetStaticMesh _hextile_collider "/Game/Geometry/Meshes/HexWall1.HexWall1"))
    (:NewEnumerator1
      (Components|StaticMesh|SetStaticMesh _hextile_collider "/Game/Geometry/Meshes/HexWall2.HexWall2"))
    (:NewEnumerator2
      (Components|StaticMesh|SetStaticMesh _hextile_collider "/Game/Geometry/Meshes/HexWall3.HexWall3"))
    (:NewEnumerator3
      (Components|StaticMesh|SetStaticMesh _hextile_collider "/Game/Geometry/Meshes/HexCorner1.HexCorner1"))
    (:NewEnumerator4
      (Components|StaticMesh|SetStaticMesh _hextile_collider "/Game/Geometry/Meshes/HexTile_Collider.HexTile_Collider"))))

(fn ConstructionScript
  (bind _hextile_collider (Variables|Components|GetHexTile_Collider))
  (switch Utilities|FlowControl|Switch|SwitchonWallTypeEnum (Variables|Default|GetWall%20Type)
    (:NewEnumerator0
      (Components|StaticMesh|SetStaticMesh _hextile_collider "/Game/Geometry/Meshes/HexWall1.HexWall1"))
    (:NewEnumerator1
      (Components|StaticMesh|SetStaticMesh _hextile_collider "/Game/Geometry/Meshes/HexWall2.HexWall2"))
    (:NewEnumerator2
      (Components|StaticMesh|SetStaticMesh _hextile_collider "/Game/Geometry/Meshes/HexWall3.HexWall3"))
    (:NewEnumerator3
      (Components|StaticMesh|SetStaticMesh _hextile_collider "/Game/Geometry/Meshes/HexCorner1.HexCorner1"))
    (:NewEnumerator4
      (Components|StaticMesh|SetStaticMesh _hextile_collider "/Game/Geometry/Meshes/HexTile_Collider.HexTile_Collider"))))
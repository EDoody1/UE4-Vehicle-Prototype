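; AI-driven wheeled vehicle Blueprint that sets up its own pathfinding on BeginPlay.
; It spawns a BP_AIPathfindingTarget at the world origin, stores it as FollowTarget and registers itself as that target's following actor.
; VehicleAIAdvancedPathfinding receives the vehicle, its left, central and right sensors, and all BP_DeathmatchWP waypoints.
; The SetPathfindingDestination call toward FollowTarget is disconnected and never runs.
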(event EventBeginPlay
  (bind _self self)
  (|CallParentFunction)
  (bind _returnvalue (Game|SpawnActorfromClass "/Game/Blueprints/BP_AIPathfindingTarget.BP_AIPathfindingTarget_C" (Math|Transform|MakeTransform "0, 0, 0") "Undefined" 0 0))
  (bind _output_get (Variables|Default|SetFollowTarget _returnvalue))
  (Variables|/Game/Blueprints/BP_AIPathfindingTarget.BP_AIPathfindingTarget_C|SetFollowingActor _output_get self)
  (bind _outactors (Actor|GetAllActorsOfClass "/Game/Blueprints/BP_DeathmatchWP.BP_DeathmatchWP_C"))
  (Class|VehicleAIAdvancedPathfinding|SetRequiredProperties (Variables|Default|GetVehicleAI_AdvancedPathfinding) _self (Variables|Default|GetLeftSensor) (Variables|Default|GetCentralSensor) (Variables|Default|GetRightSensor) _self _outactors))

(fn ConstructionScript
  (|CallParentFunction))
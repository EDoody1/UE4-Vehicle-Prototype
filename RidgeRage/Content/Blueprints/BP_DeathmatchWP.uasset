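; BP_DeathmatchWP is a placeable Deathmatch waypoint actor that can snap itself to a set height above the ground.
; While DropWaypoints is on, the Construction Script traces downward for objects with a persistent debug line and moves the actor above the hit point.
; It clears the flag once the actor sits close to that target.
; The event graph holds no active logic.
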(event EventBeginPlay)

(event Collision|EventActorBeginOverlap
  (params (OtherActor :type Actor%20Object%20Reference)))

(event EventTick
  (params (DeltaSeconds :type Float%20%28single-precision%29)))

(fn ConstructionScript
  (bind _returnvalue (Transformation|GetActorLocation))
  (if (Variables|Default|GetDrop%20Waypoints?)
    (bind (_outhit _returnvalue_2) (Collision|LineTraceForObjects _returnvalue (- _returnvalue "0, 0,500.000000") (Variables|Default|GetNewVar_0) false 0 "Persistent"))
    (if _returnvalue_2
      (Transformation|SetActorLocation self (+ (.ImpactPoint (Collision|BreakHitResult _outhit)) "0, 0,200.000000") false false)
      (if (< (Math|Vector|VectorLength (- (Transformation|GetActorLocation) (+ (.ImpactPoint (Collision|BreakHitResult _outhit)) "0, 0,200.000000"))) 1e+02)
        (Variables|Default|SetDrop%20Waypoints? false)))))
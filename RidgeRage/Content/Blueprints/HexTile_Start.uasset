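; HexTile_Start is a starting hex tile, a child Blueprint whose owning team is locked and shown by its glow color.
; Its construction script disables team changing, runs the parent script, then reads the owning team's color from the MPC_TeamColors parameter collection by a name built from the one-based team number.
; It applies that color at boosted intensity to the emissive parameter on HexTileCollider's materials.
; Runtime events only forward to the parent.
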(event EventBeginPlay
  (|CallParentFunction))

(event Collision|EventActorBeginOverlap
  (params (OtherActor :type Actor%20Object%20Reference))
  (|CallParentFunction OtherActor))

(event EventTick
  (params (DeltaSeconds :type Float%20%28single-precision%29))
  (|CallParentFunction DeltaSeconds))

(fn ConstructionScript
  (Variables|Default|SetCanChangeTeam? false)
  (|CallParentFunction)
  ;[1 1 1] Gets Color From Collection
  (bind _returnvalue (Rendering|Material|GetVectorParameterValue "/Game/Blueprints/MPC_TeamColors.MPC_TeamColors" (Utilities|Name|MakeLiteralName (Utilities|String|StringToName (Utilities|String|Append "Team" (Utilities|String|ToString(Integer) (+ (Variables|Default|GetOwningTeam) 1))))) :!class /Script/Engine.KismetMaterialLibrary))
  ;[1 1 1] Sets Color
  (Rendering|Material|SetVectorParameterValueonMaterials (Variables|Default|GetHexTile_Collider) "Emissive Color" (* (Math|Conversions|ToVector(LinearColor) _returnvalue) 2.0)))
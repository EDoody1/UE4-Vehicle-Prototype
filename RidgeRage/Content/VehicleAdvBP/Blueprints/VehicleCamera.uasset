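; Follow camera actor that becomes the first player's view target and trails the first VehicleBlueprint it finds in the level.
; BeginPlay looks up the vehicle, and Tick retries whenever that reference is invalid.
; Each tick it interpolates toward the vehicle's location, using separate speeds for horizontal follow and height.
; A per-tick debug print labelled "Cam Loc" actually shows the vehicle's location.
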(event Custom|GetPlayerLocation
  (Variables|Default|SetTargetLocation (Transformation|GetActorLocation (Variables|Default|GetPlayerVehicle))))

(event Custom|GetPlayer
  (bind _outactors (Actor|GetAllActorsOfClass "/Game/VehicleAdvBP/Blueprints/VehicleBlueprint.VehicleBlueprint_C"))
  (Variables|Default|SetPlayerVehicle (Utilities|Array|Get(acopy) _outactors)))

(event Custom|SetCameraLocation
  (bind _returnvalue (Transformation|GetActorLocation))
  (bind _delta (Variables|Default|GetDelta))
  (bind _targetlocation (Variables|Default|GetTargetLocation))
  (bind _followspeed (Variables|Default|GetFollowSpeed))
  (bind _returnvalue_2 (Class|KismetMathLibrary|TInterpto (Math|Transform|MakeTransform (Math|Vector|MakeVector (.x _returnvalue) (.y _returnvalue) (.z _returnvalue)) "0, 0, 0" "1,1,1") (Math|Transform|MakeTransform (Math|Vector|MakeVector (.x _targetlocation) (.y _targetlocation) (.z _returnvalue)) "0, 0, 0" "1,1,1") _delta _followspeed))
  (Transformation|SetActorTransform self (Math|Transform|MakeTransform (Math|Vector|MakeVector (.x (.location _returnvalue_2)) (.y (.location _returnvalue_2)) (Math|Interpolation|FInterpTo (.z _returnvalue) (.z _targetlocation) _delta (Variables|Default|GetHeightFollowSpeed))) "0, 0, 0" "1,1,1")))

(event EventBeginPlay
  (Game|Player|SetViewTargetwithBlend (Game|GetPlayerController 0) self 0.0 "VTBlend_Linear" 0.0 false)
  (bind _outactors (Actor|GetAllActorsOfClass "/Game/VehicleAdvBP/Blueprints/VehicleBlueprint.VehicleBlueprint_C"))
  (Variables|Default|SetPlayerVehicle (Utilities|Array|Get(acopy) _outactors)))

(event EventTick
  (params (DeltaSeconds :type Float%20%28single-precision%29))
  (Variables|Default|SetDelta DeltaSeconds)
  (Utilities|IsValid (Variables|Default|GetPlayerVehicle)
    (:Is%20Valid
      (CallFunction|GetPlayerLocation)
      (CallFunction|SetCameraLocation)
      (Development|PrintString (Utilities|String|Append "Cam Loc:" (Utilities|String|ToString(Vector) (Transformation|GetActorLocation (Variables|Default|GetPlayerVehicle)))) true true "(R=0.000000,G=0.660000,B=1.000000,A=1.000000)" 0.0))
    (:Is%20Not%20Valid
      (CallFunction|GetPlayer))))

(fn ConstructionScript)
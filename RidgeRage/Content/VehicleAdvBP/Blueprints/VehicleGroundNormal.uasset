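; VehicleGroundNormal is an actor that follows the player's vehicle, hovering at a fixed height above it.
; On BeginPlay it caches the first VehicleBlueprint actor found in the level, searching again on Tick whenever that reference is invalid.
; While the reference is valid, each Tick moves it to the vehicle's location plus a vertical offset, without sweeping.
; Despite the name, it computes no ground normal and leaves rotation untouched.
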(event Custom|SetLocation
  (Transformation|SetActorLocation (+ (Transformation|GetActorLocation (Variables|Default|GetPlayerVehicle)) "0, 0,150.000000") false false))

(event Custom|GetPlayer
  (bind _outactors (Actor|GetAllActorsOfClass "/Game/VehicleAdvBP/Blueprints/VehicleBlueprint.VehicleBlueprint_C"))
  (Variables|Default|SetPlayerVehicle (Utilities|Array|Get(acopy) _outactors)))

(event EventBeginPlay
  (bind _outactors (Actor|GetAllActorsOfClass "/Game/VehicleAdvBP/Blueprints/VehicleBlueprint.VehicleBlueprint_C"))
  (Variables|Default|SetPlayerVehicle (Utilities|Array|Get(acopy) _outactors)))

(event EventTick
  (params (DeltaSeconds :type Float%20%28single-precision%29))
  (Variables|Default|SetDelta DeltaSeconds)
  (Utilities|IsValid (Variables|Default|GetPlayerVehicle)
    (:Is%20Valid
      (CallFunction|SetLocation))
    (:Is%20Not%20Valid
      (CallFunction|GetPlayer))))

(fn ConstructionScript)